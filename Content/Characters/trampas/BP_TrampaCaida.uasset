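; BP_TrampaCaida is a falling trap that drops a cube and damages the player character.
; When a BP_ThirdPersonCharacter first overlaps the TriggerDetection component, a one-shot flag is set and TrapCube gains physics simulation and gravity.
; TrapCube's hit event applies fixed damage to any third-person character it strikes, with no limit on repeated hits.
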(event OnComponentBeginOverlap(TriggerDetection)
  (params (OverlappedComponent :type Primitive%20Component%20Object%20Reference) (OtherActor :type Actor%20Object%20Reference) (OtherComp :type Primitive%20Component%20Object%20Reference) (OtherBodyIndex :type Integer) (bFromSweep :type Boolean) (SweepResult :type Hit%20Result%20Structure%20%28by%20ref%29))
  (Utilities|Casting|CastToBP_ThirdPersonCharacter OtherActor)
  (if (not (Variables|Default|GetTrapTriggered))
    (Variables|Default|SetTrapTriggered true)
    (Physics|SetSimulatePhysics (Variables|Default|GetTrapCube) true)
    (Physics|SetEnableGravity (Variables|Default|GetTrapCube) true)))

(event OnComponentHit(TrapCube)
  (params (HitComponent :type Primitive%20Component%20Object%20Reference) (OtherActor :type Actor%20Object%20Reference) (OtherComp :type Primitive%20Component%20Object%20Reference) (NormalImpulse :type Vector :default "0, 0, 0") (Hit :type Hit%20Result%20Structure%20%28by%20ref%29))
  (bind _asbp_third_person_character (Utilities|Casting|CastToBP_ThirdPersonCharacter OtherActor))
  (Game|Damage|ApplyDamage _asbp_third_person_character 15.0 0 0))

(fn ConstructionScript)