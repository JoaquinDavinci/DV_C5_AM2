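; BP_A_DM is an actor that drives its Cube's color, roughness and metallic through dynamic material instances.
; BeginPlay creates an instance per material slot, saves the base color and applies the values via SetValues.
; While Inicio is true, Tick randomizes blue and alpha each frame until TiempoTotal, then restores the base color.
; IniciarTimer sets Pedido and Time, restores immediately and calls TimerFinalizado2, without setting Inicio.
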(event Custom|SetValues
  ;[0.15 0.15 0.15 0.5] Cambia de color
  (for _array_element (Variables|Default|GetMaterialInstances)
    (Rendering|Material|SetVectorParameterValue _array_element "Color2" (Variables|Default|GetColorAAsignar) :!class /Script/Engine.MaterialInstanceDynamic)
    (Rendering|Material|SetScalarParameterValue _array_element "Roughness" (Variables|Default|GetRoughness) :!class /Script/Engine.MaterialInstanceDynamic)
    (Rendering|Material|SetScalarParameterValue _array_element "Metallic" (Variables|Default|GetMetallic) :!class /Script/Engine.MaterialInstanceDynamic)))

(event Custom|TimerFinalizado
  (Development|PrintString "Timer finalizado")
  (Variables|Default|SetColorAAsignar (Variables|Default|GetColorBase))
  (CallFunction|SetValues))

(event Custom|TimerCorriendo
  (bind _returnvalue (Math|Random|RandomFloat))
  (Development|PrintString "Corriendo timer" true true "(R=0.000000,G=0.660000,B=1.000000,A=1.000000)" 0.01)
  (Variables|Default|SetColorAAsignar (Utilities|Struct|MakeLinearColor 0.0 0.0 _returnvalue _returnvalue))
  (CallFunction|SetValues))

(event EventBeginPlay
  (bind _cube (Variables|Default|GetCube))
  ;[0.15 0.15 0.15 0.5] Asigna el meterial
  (for (_array_element _array_index) (Rendering|Material|GetMaterials _cube)
    (bind _returnvalue (Rendering|Material|CreateDynamicMaterialInstance _cube _array_index _array_element "None" :!class /Script/Engine.PrimitiveComponent))
    (Utilities|Array|SetArrayElem (Variables|Default|GetMaterialInstances) _array_index _returnvalue true)
    (Variables|Default|SetColorBase (Variables|Default|GetColorAAsignar)))
  (CallFunction|SetValues))

(event EventTick
  (params (DeltaSeconds :type Float%20%28single-precision%29))
  ;[0.15 0.15 0.15 0.5] Timer
  (if (Variables|Default|GetInicio)
    (Variables|Default|SetTime (+ (Variables|Default|GetTime) (Utilities|Time|GetWorldDeltaSeconds)))
    (if (> (+ (Variables|Default|GetTime) (Utilities|Time|GetWorldDeltaSeconds)) (Variables|Default|GetTiempoTotal))
      (Variables|Default|SetTime 0.0)
      (CallFunction|TimerFinalizado)
      (Variables|Default|SetInicio false)
      (else
        (Variables|Default|SetTime (+ (Variables|Default|GetTime) (Utilities|Time|GetWorldDeltaSeconds)))
        (CallFunction|TimerCorriendo)))))

(fn ConstructionScript)

(fn IniciarTimer
  (params (Tiempo :type Float%20%28double-precision%29))
  (Variables|Default|SetPedido true)
  (Variables|Default|SetTime Tiempo)
  (CallFunction|TimerFinalizado)
  (Default|CallTimerFinalizado2))